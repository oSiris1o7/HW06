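; BP_MeshingunStudio_Info is a Meshingun studio info card for the asset pack's overview map, with a logo and text.
; Its construction script shows the card hierarchy and applies the overview theme.
; Theming finds BP_Overview_ThemeSystem, looks up its data table row by the theme enum's name, then sets the card and logo materials and text color.
; It has no active runtime logic.
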(fn `ApplyOverviewTheme`
  (bind _returnvalue (`GameplayStatics.GetActorOfClass` "/Game/FreeWastelandProps_Meshingun/Map/Overview/System/BP_Overview_ThemeSystem.BP_Overview_ThemeSystem_C"))
  (bind _returnvalue_2 (`|GetDataTableRow` (`/Game/FreeWastelandProps_Meshingun/Map/Overview/System/BP_Overview_ThemeSystem.Theme Table` _returnvalue) (`KismetStringLibrary.Conv_StringToName` (`|GetEnumeratorNameAsString` (`self.overviewTheme_Internal`))))
    (:`then`
      (bind (_categoryplatform _categorytextcolor _lightroomplatform _infocardbackground _infocardtextcolor _infocardmeshingunlogo) (break `/Game/FreeWastelandProps_Meshingun/Map/Overview/Structure/S_Overview_Theme` _returnvalue_2))
      (`PrimitiveComponent.SetMaterial` (`self.Card`) 0 _infocardbackground)
      (`PrimitiveComponent.SetMaterial` (`self.MeshingunLogo`) 0 _infocardmeshingunlogo)
      (`TextRenderComponent.SetTextRenderColor` (`self.FollowUs`) _infocardtextcolor)
      (`TextRenderComponent.SetTextRenderColor` (`self.Description`) _infocardtextcolor)
      (`TextRenderComponent.SetTextRenderColor` (`self.ReviewBold`) _infocardtextcolor))))

(fn `UserConstructionScript`
  (`SceneComponent.SetVisibility` (`self.InfoRoot`) true true)
  (`self.ApplyOverviewTheme`))